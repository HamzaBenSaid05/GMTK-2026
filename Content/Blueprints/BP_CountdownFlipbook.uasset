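; BP_CountdownFlipbook is a flipbook actor whose animation plays while the game mode's countdown timer runs.
; On BeginPlay it freezes playback, casts the game mode to BP_GameMode and binds handlers to its timer start and finish events.
; The start handler sets the RenderComponent play rate to normal speed, and the finish handler sets it back to zero, halting the animation without rewinding it.
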(event `self.ReceiveBeginPlay`
  (`PaperFlipbookComponent.SetPlayRate` (`self.RenderComponent`) 0.0)
  (bind _asbp_game_mode (cast `/Game/Blueprints/BP_GameMode` (`GameplayStatics.GetGameMode`)))
  (add `GMTK_GameMode.OnTimerStart` _asbp_game_mode (delegate `StartCountDown`))
  (add `GMTK_GameMode.OnTimerFinish` _asbp_game_mode (delegate `FinishCountDown`)))

(event `StartCountDown`
  (`PaperFlipbookComponent.SetPlayRate` (`self.RenderComponent`) 1.0))

(event `FinishCountDown`
  (`PaperFlipbookComponent.SetPlayRate` (`self.RenderComponent`) 0.0))

(fn `UserConstructionScript`)