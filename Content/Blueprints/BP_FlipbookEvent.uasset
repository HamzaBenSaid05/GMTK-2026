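; BP_FlipbookEvent is a flipbook actor that can switch its displayed animation by event tag.
; On BeginPlay it finds the BP_SceneController and binds an event to its state-changed notification.
; ChangeFlipbook checks the Flipbooks map for the given tag, then loops over the map to set the matching entry on the RenderComponent.
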(event `self.ReceiveBeginPlay`
  (bind _returnvalue (`GameplayStatics.GetActorOfClass` "/Game/Blueprints/BP_SceneController.BP_SceneController_C"))
  (bind _output_get (set `self.SceneController` _returnvalue))
  (add `GMTK_SceneControllerBase.OnStateChanged` _output_get (`|CreateDelegate` :!event `ChangeFlipbook`)))

(fn `ChangeFlipbook`
  (params (EventTag :type "GameplayTag Structure"))
  (if (`.ReturnValue` (`BlueprintMapLibrary.Map_Find` (`self.Flipbooks`) EventTag))
    (bind (_keypin _valuepin) (`|MapForEach` (`self.Flipbooks`))
      (:`then`
        (if (== _keypin (`local.EventTag`))
          (`PaperFlipbookComponent.SetFlipbook` (`self.RenderComponent`) (`|ConvertAsset` _valuepin)))))))

(fn `UserConstructionScript`)