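; BP_PlayerControllerFinal is a player controller that presents the WBP_FinalNotes widget and lets the player try to ignite a lighter within it.
; On BeginPlay it creates and stores the widget, adds it to the viewport, registers the IMC_Mouse Enhanced Input context and hides the mouse cursor.
; The IA_Interact action forwards to TryIgnite on the widget's nested LighterWidget, so the controller only routes input to the UI.
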(event `self.ReceiveBeginPlay`
  (bind _returnvalue (`|CreateWidget` "/Game/Blueprints/UI/WBP_FinalNotes.WBP_FinalNotes_C" self))
  (bind _output_get (set `self.FinalNotesWidget` _returnvalue))
  (`UserWidget.AddToViewport` _output_get 0)
  (message `EnhancedInputSubsystemInterface.AddMappingContext` (subsystem `EnhancedInputLocalPlayerSubsystem`) "/Game/Input/IMC_Mouse.IMC_Mouse" 0 (struct))
  (set `self.bShowMouseCursor` false))

(event `EnhancedInput|/Game/Input/Actions/IA_Interact`
  (params (ActionValue :type Boolean) (ElapsedSeconds :type "Float (double-precision)") (TriggeredSeconds :type "Float (double-precision)") (InputAction :type "InputAction Object Reference" :default "/Game/Input/Actions/IA_Interact.IA_Interact"))
  (:`Triggered`
    (`GMTK_LighterWidget.TryIgnite` (`GMTK_FinalNotesWidget.LighterWidget` (`self.FinalNotesWidget`)))))

(fn `UserConstructionScript`)