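; Weather event actor that swaps the ambient sound and particle effect whenever a WeatherEvent fires with a new weather type.
; It looks up the sound and emitter for that weather in maps, fading out and later destroying the old audio component while a new one fades in, producing a crossfade.
; The previous effect is deactivated and the new emitter spawns attached to the first player pawn's root component.
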(event `/Game/StylizedWeather/Blueprint/BPI_WeatherEvent.WeatherEvent`
  (params (Weather :type "/Game/StylizedWeather/Blueprint/Enum_Weaher Enum" :default "NewEnumerator0"))
  (bind _sound_fade_out_duration (`self.Sound Fade Out Duration`))
  (`|ExecutionSequence`
    (:`then_0`
      (bind _audio (`self.Audio`)
        (:`then`
          (`|ExecutionSequence`
            (:`then_0`
              (bind _output_get (set `self.Audio_Buf` _audio))
              (`AudioComponent.FadeOut` _output_get _sound_fade_out_duration 0.0 "Linear")
              (`KismetSystemLibrary.Delay` _sound_fade_out_duration)
              (`ActorComponent.K2_DestroyComponent` (`self.Audio_Buf`)))
            (:`then_1`
              (bind _returnvalue (`AddComponent|NODE_AddAudioComponent-0` :!label _label))
              (bind _output_get_2 (set `self.Audio` _returnvalue))
              (`AudioComponent.SetSound` _output_get_2 (`BlueprintMapLibrary.Map_Find` (`self.Sound`) Weather))
              (`AudioComponent.FadeIn` _output_get_2 (`self.Sound Fade In Duration`) 1.0 0.0 "Linear"))))
        (:`else`
          (goto _label))))
    (:`then_1`
      (bind _effect (`self.Effect`)
        (:`then`
          (`ActorComponent.Deactivate` _effect))
        (:`else`
          _))
      (bind _returnvalue_2 (`GameplayStatics.SpawnEmitterAttached` (`BlueprintMapLibrary.Map_Find` (`self.Effects`) Weather) (`Actor.RootComponent` (`GameplayStatics.GetPlayerPawn` 0)) "None" (0.0 0.0 0.0) (struct) (1.0 1.0 1.0) "SnapToTarget"))
      (set `self.Effect` _returnvalue_2))))

(fn `UserConstructionScript`
  (`parent.UserConstructionScript`))